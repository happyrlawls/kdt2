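; Test actor, BP_HelloActor, meant to move its Sphere component back and forth along X.
; Each Tick sets the Sphere's relative X to Speed times DeltaSeconds, negated when Ismoveright is false, rather than adding it to the current position.
; World X thresholds flip Ismoveright to reverse direction.
; The construction script and an extra function are empty.
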(event `self.ReceiveTick`
  (params (DeltaSeconds :type "Float (single-precision)"))
  (bind _sphere (`self.Sphere`))
  (bind _sphere_2 (`self.Sphere`))
  (bind _returnvalue_x (`KismetMathLibrary.BreakVector` (`SceneComponent.K2_GetComponentLocation` _sphere)))
  (bind _returnvalue_x_2 (`KismetMathLibrary.BreakVector` (`SceneComponent.K2_GetComponentLocation` _sphere_2)))
  (if (`self.ismoveright`)
    ;[0.2311 0.3032 1] 오른쪽으로 이동
    (`SceneComponent.K2_SetRelativeLocation` _sphere_2 (`KismetMathLibrary.MakeVector` (* DeltaSeconds (`self.speed`))) false false)
    (if (>= _returnvalue_x_2 500.0)
      (set `self.ismoveright` false))
    (else
      ;[1 0.8673 0] 왼쪽으로 이동
      (`SceneComponent.K2_SetRelativeLocation` _sphere (`KismetMathLibrary.MakeVector` (* (* DeltaSeconds (`self.speed`)) -1.0)) false false)
      (if (<= _returnvalue_x 0.0)
        (set `self.ismoveright` true)))))

(fn `UserConstructionScript`)

(fn `새 함수`)